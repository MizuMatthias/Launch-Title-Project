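; Ice wall that melts on heat by sliding its cube along Z with the Displacement timeline, scaled by DisplacementValue.
; Hot water contact plays the displacement and restarts the UnmeltDelay timeline, used as a MeltedTime-based timer that reverses the melt when finished.
; Temperature interactions drive the same timeline directly, forward for Hot and back for Neutral, without the timer.
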(event EventBeginPlay)

(event Collision|EventActorBeginOverlap
  (params (OtherActor :type Actor%20Object%20Reference)))

(event EventTick
  (params (DeltaSeconds :type Float%20%28single-precision%29)))

(event EventTempInteraction
  (params (Attribute :type Enum_Temperatures%20Enum :default "NewEnumerator0"))
  (switch Utilities|FlowControl|Switch|SwitchonEnum_Temperatures Attribute
    (:NewEnumerator0
      (bind _newtrack_0 (Timeline|Displacement Reverse)
        (:Update
          (Transformation|SetRelativeLocation (Variables|Default|GetCube) (Math|Vector|MakeVector 0.0 0.0 (* _newtrack_0 (Variables|Default|GetDisplacementValue))) false false))))
    (:NewEnumerator1
      (Timeline|Displacement Play))))

(event EventWaterContact
  (params (Attribute :type Enum_Temperatures%20Enum :default "NewEnumerator0"))
  (switch Utilities|FlowControl|Switch|SwitchonEnum_Temperatures Attribute
    (:NewEnumerator1
      (Utilities|FlowControl|Sequence
        (:then_0
          (Timeline|UnmeltDelay PlayFromStart
            (:Finished
              (bind _newtrack_0 (Timeline|Displacement Reverse)
                (:Update
                  (Transformation|SetRelativeLocation (Variables|Default|GetCube) (Math|Vector|MakeVector 0.0 0.0 (* _newtrack_0 (Variables|Default|GetDisplacementValue))) false false))))))
        (:then_1
          (Timeline|UnmeltDelay SetNewTime))
        (:then_2
          (Timeline|Displacement Play))))))

(fn ConstructionScript)