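; BP_Lumiflora is a glowing plant that grows on water contact and triggers growth in photo plants within its radius.
; GrowthLevel scales its mesh, collision sphere, decal and light intensity.
; Each watering below full growth restarts a chain of Stable, Fluctuating, Waning and Dying timelines that modulate the light, with Dying shrinking the plant.
; Sphere overlaps set IsLit on BP_PhotoPlant_Parent actors, starting or reversing their growth.
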(event OnComponentBeginOverlap(Sphere)
  (params (OverlappedComponent :type Primitive%20Component%20Object%20Reference) (OtherActor :type Actor%20Object%20Reference) (OtherComp :type Primitive%20Component%20Object%20Reference) (OtherBodyIndex :type Integer) (bFromSweep :type Boolean) (SweepResult :type Hit%20Result%20Structure%20%28by%20ref%29))
  ;[1 1 1] Detects when plant becomes In or Out of range
  (bind _asbp_photo_plant_parent (Utilities|Casting|CastToBP_PhotoPlant_Parent OtherActor))
  (Variables|/Game/Blueprints/BP_PhotoPlant_Parent.BP_PhotoPlant_Parent_C|SetisLit? _asbp_photo_plant_parent true)
  (Default|StartGrowth _asbp_photo_plant_parent))

(event OnComponentEndOverlap(Sphere)
  (params (OverlappedComponent :type Primitive%20Component%20Object%20Reference) (OtherActor :type Actor%20Object%20Reference) (OtherComp :type Primitive%20Component%20Object%20Reference) (OtherBodyIndex :type Integer))
  ;[1 1 1] Detects when plant becomes In or Out of range
  (bind _asbp_photo_plant_parent (Utilities|Casting|CastToBP_PhotoPlant_Parent OtherActor))
  (Variables|/Game/Blueprints/BP_PhotoPlant_Parent.BP_PhotoPlant_Parent_C|SetisLit? _asbp_photo_plant_parent false)
  (Default|ReverseGrowth _asbp_photo_plant_parent))

(event Custom|LumifloraGrowth
  (bind _growthlevel (Variables|Default|GetGrowthLevel))
  ;[1 1 1] Set Scale of Lumiflora and Sphere collision
  (Transformation|SetRelativeTransform (Variables|Default|GetStaticMesh) (Math|Transform|MakeTransform (Math|Vector|MakeVector -1e+01 -1e+01 (+ (* _growthlevel 1e+02) -1e+02)) "0, 0, 0" (Math|Conversions|ToVector(Float) (+ (* _growthlevel 0.2) 0.8))) true false)
  (Components|Sphere|SetSphereRadius (Variables|Default|GetSphere) (* (Variables|Default|GetGrowthLevel) 1e+03) true)
  (Transformation|SetRelativeScale3D (Variables|Default|GetDecal) (Math|Conversions|ToVector(Float) (* (Variables|Default|GetGrowthLevel) 1e+01))))

(event Collision|EventActorBeginOverlap
  (params (OtherActor :type Actor%20Object%20Reference)))

(event EventWaterContact
  (bind _timer (Variables|Default|GetTimer))
  (bind _returnvalue (- _timer 3.0))
  (bind _returnvalue_2 (/ _returnvalue 2.0))
  (bind _returnvalue_3 (- 3e+01 _returnvalue_2))
  ;[1 1 1] Detect water contact
  (if (< (Variables|Default|GetGrowthLevel) 1.0)
    (bind _output_get (Variables|Default|SetGrowthLevel (+ (Variables|Default|GetGrowthLevel) 0.01)))
    (Variables|Default|SetGrowthPeak _output_get)
    (CallFunction|LumifloraGrowth)
    ;[1 1 1] Light intensity Fluctuation
    (Utilities|FlowControl|Sequence
      (:then_0
        (bind _fluctuating (Timeline|Stable SetNewTime)
          (:Update
            (Variables|Default|SetFluctuationMultiplier _fluctuating)
            (Rendering|Components|Light|SetIntensity (Variables|Default|GetPointLight) (+ (* (* (Variables|Default|GetGrowthLevel) (Variables|Default|GetFluctuationMultiplier)) 1.195e+04) 5e+01) :!label _label))
          (:Finished
            (Utilities|FlowControl|Sequence
              (:then_0
                (bind _fluctuating_2 (Timeline|Fluctuating SetNewTime)
                  (:Update
                    (Variables|Default|SetFluctuationMultiplier _fluctuating_2)
                    (goto _label))
                  (:Finished
                    (bind _fluctuating_3 (Timeline|Waning PlayFromStart)
                      (:Update
                        (Variables|Default|SetFluctuationMultiplier _fluctuating_3)
                        (goto _label))
                      (:Finished
                        (Utilities|FlowControl|Sequence
                          (:then_0
                            (bind _dying (Timeline|Dying SetNewTime)
                              (:Update
                                (Variables|Default|SetFluctuationMultiplier _dying)
                                ;[1 1 1] Reverse Growth
                                (Variables|Default|SetGrowthLevel (Math|Float|Clamp(Float) (* _dying (Variables|Default|GetFluctuationMultiplier) 0.5) 0.0 (Variables|Default|GetGrowthPeak)))
                                (CallFunction|LumifloraGrowth)
                                (goto _label))))
                          (:then_1
                            (Timeline|Dying Play))))))))
              (:then_1
                (Timeline|Fluctuating Play))))))
      (:then_1
        (Timeline|Stable Play))
      (:then_2
        (Timeline|Fluctuating Stop))
      (:then_3
        (Timeline|Waning Stop))
      (:then_4
        (Timeline|Dying Stop)))))

(event EventBeginPlay
  (bind _growthlevel (Variables|Default|GetGrowthLevel))
  ;[1 1 1] Set scale on game start
  (Rendering|Components|Light|SetIntensity (Variables|Default|GetPointLight) 0.0)
  ;[1 1 1] Set Scale of Lumiflora and Sphere collision
  (Transformation|SetRelativeTransform (Variables|Default|GetStaticMesh) (Math|Transform|MakeTransform (Math|Vector|MakeVector -1e+01 -1e+01 (+ (* _growthlevel 1e+02) -1e+02)) "0, 0, 0" (Math|Conversions|ToVector(Float) (+ (* _growthlevel 0.2) 0.8))) true false)
  (Components|Sphere|SetSphereRadius (Variables|Default|GetSphere) (* (Variables|Default|GetGrowthLevel) 1e+03) true)
  (Transformation|SetRelativeScale3D (Variables|Default|GetDecal) (Math|Conversions|ToVector(Float) (* (Variables|Default|GetGrowthLevel) 1e+01))))

(fn ConstructionScript)