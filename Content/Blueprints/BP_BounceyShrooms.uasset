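; BP_BounceyShrooms is a bouncy mushroom pad that launches the player character when they touch it.
; On sphere overlap it launches the cached third-person character along the arrow's forward vector, overriding velocity, and resets their air control, gravity scale and rope reference.
; It also plays a cartoon boing sound and runs a timeline that squashes and stretches the cylinder's height.
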(event OnComponentBeginOverlap(Sphere)
  (params (OverlappedComponent :type Primitive%20Component%20Object%20Reference) (OtherActor :type Actor%20Object%20Reference) (OtherComp :type Primitive%20Component%20Object%20Reference) (OtherBodyIndex :type Integer) (bFromSweep :type Boolean) (SweepResult :type Hit%20Result%20Structure%20%28by%20ref%29))
  (bind _as_bp_third_person_character (Variables|Default|GetAs%20BP%20Third%20Person%20Character))
  (bind _charactermovement (Variables|/Script/Engine.Character|GetCharacterMovement _as_bp_third_person_character))
  (if (== OtherActor _as_bp_third_person_character)
    (Character|LaunchCharacter _as_bp_third_person_character (* (Math|Vector|GetForwardVector (Variables|Default|GetArrow)) (Variables|Default|GetLaunchStrength)) true true)
    (Variables|/Script/Engine.CharacterMovementComponent|SetAirControl _charactermovement 0.25)
    (Variables|/Script/Engine.CharacterMovementComponent|SetGravityScale _charactermovement 1.6)
    (Variables|/Game/ThirdPerson/Blueprints/BP_ThirdPersonCharacter.BP_ThirdPersonCharacter_C|SetRope%20Actor _as_bp_third_person_character 0)
    (Audio|PlaySoundatLocation "/Game/Assets/Sound/Puzzles/161122__reelworldstudio__cartoon-boing_Cue.161122__reelworldstudio__cartoon-boing_Cue" (Transformation|GetActorLocation) "0, 0, 0" 1.0 1.0 0.2 0 0 0 0)
    (bind _newtrack_0 (Timeline|Bounce PlayFromStart)
      (:Update
        (Transformation|SetRelativeScale3D (Variables|Default|GetCylinder) (Math|Vector|MakeVector 0.25 0.25 _newtrack_0))))))

(event EventBeginPlay
  (bind _asbp_third_person_character (Utilities|Casting|CastToBP_ThirdPersonCharacter (Game|GetPlayerCharacter 0)))
  (Variables|Default|SetAs%20BP%20Third%20Person%20Character _asbp_third_person_character))

(event Collision|EventActorBeginOverlap
  (params (OtherActor :type Actor%20Object%20Reference)))

(event EventTick
  (params (DeltaSeconds :type Float%20%28single-precision%29)))

(fn ConstructionScript)