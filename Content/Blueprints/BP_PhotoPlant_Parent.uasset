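; BP_PhotoPlant_Parent is the base Blueprint for plants that grow and can be moved between pots and plant spots.
; A timeline drives GrowthLevel and calls UpdateGrowth, an empty hook like WaterContact, presumably for children to override.
; GrownByDefault plants play growth on BeginPlay; others grow or reverse through StartGrowth and ReverseGrowth.
; PlantPickup and PlantPlant handle attachment, repositioning and the plant, pot and spot references.
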(event Custom|StartGrowth
  (if (not (Variables|Default|GetGrownByDefault?))
    (bind _newtrack_0 (Timeline|GrowthTimeline Play)
      (:Update
        (Variables|Default|SetGrowthLevel _newtrack_0)
        (CallFunction|UpdateGrowth)))))

(event Custom|ReverseGrowth
  (if (not (Variables|Default|GetGrownByDefault?))
    (bind _newtrack_0 (Timeline|GrowthTimeline Reverse)
      (:Update
        (Variables|Default|SetGrowthLevel _newtrack_0)
        (CallFunction|UpdateGrowth)))))

(event Custom|Update%20Growth)

(event EventPlantPickup
  (params (PotToAttach :type BP%20Plant%20Pot%20Object%20Reference))
  (Variables|Default|SetAttachedPot PotToAttach)
  (Transformation|AttachComponentToComponent (Variables|/Game/Blueprints/BP_PlantPot.BP_PlantPot_C|GetCylinder (Variables|Default|GetAttachedPot)) "None" "KeepWorld" "KeepWorld" "KeepWorld" false)
  (Transformation|SetActorLocation (Math|Vector|MakeVector (.x (Transformation|GetActorLocation (Variables|Default|GetAttachedPot))) (.y (Transformation|GetActorLocation (Variables|Default|GetAttachedPot))) (+ (.z (Transformation|GetActorLocation (Variables|Default|GetAttachedPot))) 1e+02)) false false)
  (Variables|/Game/Blueprints/BP_PlantPot.BP_PlantPot_C|SetHasPlant? (Variables|Default|GetAttachedPot) true)
  (Variables|/Game/Blueprints/BP_PlantPot.BP_PlantPot_C|SetPlant_REF (Variables|Default|GetAttachedPot) self)
  (Variables|Default|SetPlantSpot 0))

(event Collision|EventActorBeginOverlap
  (params (OtherActor :type Actor%20Object%20Reference)))

(event EventTick
  (params (DeltaSeconds :type Float%20%28single-precision%29)))

(event EventWaterContact
  (params (Attribute :type Enum_Temperatures%20Enum :default "NewEnumerator0")))

(event EventBeginPlay
  (bind _asbp_third_person_character (Utilities|Casting|CastToBP_ThirdPersonCharacter (Game|GetPlayerCharacter 0)))
  (Variables|Default|SetPlayer_REF _asbp_third_person_character)
  (if (Variables|Default|GetGrownByDefault?)
    (bind _newtrack_0 (Timeline|GrowthTimeline Play)
      (:Update
        (Variables|Default|SetGrowthLevel _newtrack_0)
        (CallFunction|UpdateGrowth)))))

(event EventPlantPlant
  (params (PlantSpot :type BP%20Plant%20Spot%20Object%20Reference))
  (Variables|Default|SetPlantSpot PlantSpot)
  (Transformation|DetachFromComponent (Variables|/Game/Blueprints/BP_PlantPot.BP_PlantPot_C|GetCylinder (Variables|Default|GetAttachedPot)) "KeepWorld" "KeepWorld" "KeepWorld" true)
  (Transformation|SetActorLocation (Transformation|GetActorLocation (Variables|Default|GetPlantSpot)) false false)
  (Variables|/Game/Blueprints/BP_PlantPot.BP_PlantPot_C|SetHasPlant? (Variables|Default|GetAttachedPot) false)
  (Variables|/Game/Blueprints/BP_PlantPot.BP_PlantPot_C|SetPlant_REF (Variables|Default|GetAttachedPot) 0)
  (Variables|Default|SetAttachedPot 0))

(fn ConstructionScript)