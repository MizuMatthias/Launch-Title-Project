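; BP_Rope is a swingable rope actor that the player grabs on contact.
; When its Capsule overlaps an actor that answers IsPlayerMessage, it sends GrabRopeMessage with itself and lowers TestSphere's linear damping so it swings freely.
; AddSwingingForce pushes TestSphere as an acceleration, and Rest raises damping again to settle it.
; The Growth event is an empty stub.
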(event OnComponentBeginOverlap(Capsule)
  (params (OverlappedComponent :type Primitive%20Component%20Object%20Reference) (OtherActor :type Actor%20Object%20Reference) (OtherComp :type Primitive%20Component%20Object%20Reference) (OtherBodyIndex :type Integer) (bFromSweep :type Boolean) (SweepResult :type Hit%20Result%20Structure%20%28by%20ref%29))
  (bind _true_ (Class|BPIPlayer|IsPlayer?(Message) OtherActor))
  (if _true_
    (Class|BPIPlayer|GrabRope(Message) OtherActor self)
    (Class|PrimitiveComponent|SetLinearDamping (Variables|Default|GettestSphere) 0.05)))

(event Custom|AddSwingingForce
  (params (Force :type Vector))
  (Physics|AddForce (Variables|Default|GettestSphere) Force "None" true))

(event Custom|Rest
  (Class|PrimitiveComponent|SetLinearDamping (Variables|Default|GettestSphere) 2.0))

(event EventBeginPlay)

(event Collision|EventActorBeginOverlap
  (params (OtherActor :type Actor%20Object%20Reference)))

(event EventGrowth)

(fn ConstructionScript)