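; Temperature plant actor that applies its Hot, Cold or Neutral temperature to actors entering its radius.
; The construction script selects material and decal color from Temperature, also swapping the mesh for Hot and Cold.
; BeginPlay and UpdateGrowth scale the mesh, trigger sphere and decal from GrowthLevel, with sphere and decal offset by half a level.
; Sphere overlaps send TempInteractionMessage with the plant's temperature on entry and Neutral on exit.
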(event OnComponentBeginOverlap(Sphere)
  (params (OverlappedComponent :type Primitive%20Component%20Object%20Reference) (OtherActor :type Actor%20Object%20Reference) (OtherComp :type Primitive%20Component%20Object%20Reference) (OtherBodyIndex :type Integer) (bFromSweep :type Boolean) (SweepResult :type Hit%20Result%20Structure%20%28by%20ref%29))
  (Class|BPITemperature|TempInteraction(Message) OtherActor (Variables|Default|GetTemperature)))

(event OnComponentEndOverlap(Sphere)
  (params (OverlappedComponent :type Primitive%20Component%20Object%20Reference) (OtherActor :type Actor%20Object%20Reference) (OtherComp :type Primitive%20Component%20Object%20Reference) (OtherBodyIndex :type Integer))
  (Class|BPITemperature|TempInteraction(Message) OtherActor "NewEnumerator0"))

(event EventUpdateGrowth
  (bind _growthlevel (Variables|Default|GetGrowthLevel))
  (bind _returnvalue (- _growthlevel 0.5))
  (Transformation|SetRelativeTransform (Variables|Default|GetCube) (Math|Transform|MakeTransform (Math|Vector|MakeVector 0.0 0.0 0.0) "0, 0, 0" (Math|Conversions|ToVector(Float) (+ (* (Variables|Default|GetGrowthLevel) 0.8) 0.2))) true false)
  (Components|Sphere|SetSphereRadius (Variables|Default|GetSphere) (* _returnvalue (Variables|Default|GetMaxRadius)) true)
  (Transformation|SetRelativeScale3D (Variables|Default|GetDecal) (Math|Conversions|ToVector(Float) (* _returnvalue 3e+01))))

(event Collision|EventActorBeginOverlap
  (params (OtherActor :type Actor%20Object%20Reference))
  (|CallParentFunction OtherActor) ; This node is disabled and will not be called.\nDrag off pins to build functionality.
)

(event EventTick
  (params (DeltaSeconds :type Float%20%28single-precision%29))
  (|CallParentFunction DeltaSeconds) ; This node is disabled and will not be called.\nDrag off pins to build functionality.
)

(event EventBeginPlay
  (bind _growthlevel (Variables|Default|GetGrowthLevel))
  (bind _returnvalue (- _growthlevel 0.5))
  (|CallParentFunction)
  (Transformation|SetRelativeTransform (Variables|Default|GetCube) (Math|Transform|MakeTransform (Math|Vector|MakeVector 0.0 0.0 0.0) "0, 0, 0" (Math|Conversions|ToVector(Float) (+ (* (Variables|Default|GetGrowthLevel) 0.8) 0.2))) true false)
  (Components|Sphere|SetSphereRadius (Variables|Default|GetSphere) (* _returnvalue (Variables|Default|GetMaxRadius)) true)
  (Transformation|SetRelativeScale3D (Variables|Default|GetDecal) (Math|Conversions|ToVector(Float) (* _returnvalue 3e+01))))

(fn ConstructionScript
  (bind _cube (Variables|Default|GetCube))
  (bind _cube_2 (Variables|Default|GetCube))
  (|CallParentFunction)
  (switch Utilities|FlowControl|Switch|SwitchonEnum_Temperatures (Variables|Default|GetTemperature)
    (:NewEnumerator0
      (Rendering|Material|SetMaterial (Variables|Default|GetCube) 0 "/Engine/VREditor/BasicMeshes/MI_Cube_01.MI_Cube_01")
      (Rendering|Components|Decal|SetDecalMaterial (Variables|Default|GetDecal) "/Game/Materials/MI_WhiteLight.MI_WhiteLight"))
    (:NewEnumerator1
      (Components|StaticMesh|SetStaticMesh _cube_2 "/Engine/BasicShapes/Cube.Cube")
      (Rendering|Material|SetMaterial _cube_2 0 "/Engine/VREditor/BasicMeshes/MI_Cube_03.MI_Cube_03")
      (Rendering|Components|Decal|SetDecalMaterial (Variables|Default|GetDecal) "/Game/Materials/MI_RedLight.MI_RedLight"))
    (:NewEnumerator2
      (Components|StaticMesh|SetStaticMesh _cube "/Engine/BasicShapes/Sphere.Sphere")
      (Rendering|Material|SetMaterial _cube 0 "/Engine/VREditor/BasicMeshes/MI_Cube_02.MI_Cube_02")
      (Rendering|Components|Decal|SetDecalMaterial (Variables|Default|GetDecal) "/Game/Materials/MI_BlueLight.MI_BlueLight"))))